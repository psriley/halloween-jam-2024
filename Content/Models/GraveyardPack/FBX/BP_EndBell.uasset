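; BP_EndBell is an interactable bell that asks the game mode to check whether all graves are correct.
; Overlapping InteractBox stores the BP_MainGuy player, registers the bell as its interacting actor and shows the interact prompt.
; Leaving hides the prompt but sets the interacting actor to the bell again rather than clearing it.
; Interact casts to BP_FirstPersonGameMode and calls AreAllGravesCorrect, leaving any outcome to the game mode.
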(event OnComponentBeginOverlap(InteractBox)
  (params (OverlappedComponent :type Primitive%20Component%20Object%20Reference) (OtherActor :type Actor%20Object%20Reference) (OtherComp :type Primitive%20Component%20Object%20Reference) (OtherBodyIndex :type Integer) (bFromSweep :type Boolean) (SweepResult :type Hit%20Result%20Structure%20%28by%20ref%29))
  (bind _asbp_main_guy (Utilities|Casting|CastToBP_MainGuy OtherActor))
  (Variables|Default|Setplayer _asbp_main_guy)
  (Variables|/Game/Blueprints/BP_MainGuy.BP_MainGuy_C|SetInteractingActor _asbp_main_guy self)
  (Default|ShowInteract _asbp_main_guy))

(event OnComponentEndOverlap(InteractBox)
  (params (OverlappedComponent :type Primitive%20Component%20Object%20Reference) (OtherActor :type Actor%20Object%20Reference) (OtherComp :type Primitive%20Component%20Object%20Reference) (OtherBodyIndex :type Integer))
  (bind _asbp_main_guy (Utilities|Casting|CastToBP_MainGuy OtherActor))
  (Variables|/Game/Blueprints/BP_MainGuy.BP_MainGuy_C|SetInteractingActor _asbp_main_guy self)
  (Default|HideInteract _asbp_main_guy))

(event EventBeginPlay)

(event Collision|EventActorBeginOverlap
  (params (OtherActor :type Actor%20Object%20Reference)))

(event EventTick
  (params (DeltaSeconds :type Float%20%28single-precision%29)))

(event EventInteract
  (bind _asbp_first_person_game_mode (Utilities|Casting|CastToBP_FirstPersonGameMode (Game|GetGameMode)))
  (Default|AreAllGravesCorrect _asbp_first_person_game_mode))

(fn ConstructionScript)