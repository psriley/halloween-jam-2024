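; BP_MainGuy is the player character, handling the interact prompt and NPC dialogue.
; ShowInteract and HideInteract toggle the HUD prompt and the CanInteract flag that gates IA_Interact.
; A dialogue-state switch starts the interaction by freezing movement and blending the camera to the NPC, then advances lines through the NPC's ProgressDialogue.
; Once done, it restores camera, walking and NPC trigger collision, then hides the dialogue box.
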(event Custom|returnCamera
  ;[1 1 1] Returns the main camera to the mainGuy's camera
  (Game|Player|SetViewTargetwithBlend (Game|GetPlayerController 0) self 0.0 "VTBlend_Linear" 0.0 false)
  (Pawn|Components|CharacterMovement|SetMovementMode (Variables|Character|GetCharacterMovement) "MOVE_Walking" 0)
  (bind _asbp_npc (Utilities|Casting|CastToBP_NPC (Variables|Default|GetInteractingActor)))
  (Collision|SetCollisionEnabled (Variables|/Game/Blueprints/BP_NPC.BP_NPC_C|GetInteractBox _asbp_npc) "QueryOnly")
  (Variables|Default|SetcanInteract false))

(event Custom|ShowInteract
  ;[1 1 1] Show  "press e" tooltip
  (Widget|SetVisibility (Variables|/Game/Blueprints/WBP_HUD.WBP_HUD_C|Gettxt_Interact (Variables|Default|GetwidgetHUD)) "Visible")
  (Variables|Default|SetcanInteract true))

(event Custom|HideInteract
  ;[1 1 1] Hide "press e" tooltip
  (Widget|SetVisibility (Variables|/Game/Blueprints/WBP_HUD.WBP_HUD_C|Gettxt_Interact (Variables|Default|GetwidgetHUD)) "Hidden")
  (Variables|Default|SetcanInteract false))

(event Input|EnhancedActionEvents|EnhancedInputActionIA_Interact
  (params (ActionValue :type Boolean) (ElapsedSeconds :type Float%20%28double-precision%29) (TriggeredSeconds :type Float%20%28double-precision%29) (InputAction :type Input%20Action%20Object%20Reference :default "/Game/Blueprints/Input/IA_Interact.IA_Interact"))
  (bind _interactingactor (Variables|Default|GetInteractingActor))
  ;[1 1 1] Interact with NPC
  (if (Variables|Default|GetcanInteract)
    (bind _asbp_npc (Utilities|Casting|CastToBP_NPC _interactingactor)
      (:then
        (switch Utilities|FlowControl|Switch|SwitchonEDialogueState (Variables|Default|GetcurDialogueState)
          (:NewEnumerator0
            (Class|BPIInteractable|Interact(Message) _interactingactor :!label _label)
            (bind _asbp_npc_2 (Utilities|Casting|CastToBP_NPC _interactingactor))
            (Variables|Default|SetactiveNPC true)
            (Pawn|Components|CharacterMovement|DisableMovement (Variables|Character|GetCharacterMovement))
            (Game|Player|SetViewTargetwithBlend (Game|GetPlayerController 0) _asbp_npc_2 0.5 "VTBlend_Linear" 0.0 false))
          (:NewEnumerator1
            (bind _dialoguecomplete (Default|ProgressDialogue _asbp_npc self))
            (if _dialoguecomplete
              (Variables|Default|SetcurDialogueState "NewEnumerator2")))
          (:NewEnumerator2
            (CallFunction|ReturnCamera)
            (Variables|Default|SetcurDialogueState "NewEnumerator0")
            (Widget|SetVisibility (Variables|/Game/Blueprints/WBP_HUD.WBP_HUD_C|GetdialogueBox (Variables|Default|GetwidgetHUD)) "Hidden"))))
      (:CastFailed
        (goto _label)))))

(event EventBeginPlay)

(event Collision|EventActorBeginOverlap
  (params (OtherActor :type Actor%20Object%20Reference)))

(event EventTick
  (params (DeltaSeconds :type Float%20%28single-precision%29)))

(fn ConstructionScript
  (|CallParentFunction))