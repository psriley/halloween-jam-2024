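; Interactable grave plot that the player digs and then fills to bury the active NPC.
; Overlapping InteractBox registers it with BP_MainGuy, and Interact advances GraveState by toggling hole, mesh and tombstone, needing an active NPC to fill.
; Once filled, it stops offering interaction on overlap, has BP_FirstPersonGameMode check GraveID against the current NPC ID, and spawns another NPC.
; The construction script displays GraveID on the ID text.
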(event OnComponentBeginOverlap(InteractBox)
  (params (OverlappedComponent :type Primitive%20Component%20Object%20Reference) (OtherActor :type Actor%20Object%20Reference) (OtherComp :type Primitive%20Component%20Object%20Reference) (OtherBodyIndex :type Integer) (bFromSweep :type Boolean) (SweepResult :type Hit%20Result%20Structure%20%28by%20ref%29))
  (if (not (== (Variables|Default|GetgraveState) 2))
    (bind _asbp_main_guy (Utilities|Casting|CastToBP_MainGuy OtherActor))
    (Variables|Default|Setplayer _asbp_main_guy)
    (Variables|/Game/Blueprints/BP_MainGuy.BP_MainGuy_C|SetInteractingActor _asbp_main_guy self)
    (Variables|/Game/Blueprints/BP_MainGuy.BP_MainGuy_C|SetcanInteract _asbp_main_guy true)
    (Default|ShowInteract _asbp_main_guy)))

(event OnComponentEndOverlap(InteractBox)
  (params (OverlappedComponent :type Primitive%20Component%20Object%20Reference) (OtherActor :type Actor%20Object%20Reference) (OtherComp :type Primitive%20Component%20Object%20Reference) (OtherBodyIndex :type Integer))
  (bind _asbp_main_guy (Utilities|Casting|CastToBP_MainGuy OtherActor))
  (Variables|/Game/Blueprints/BP_MainGuy.BP_MainGuy_C|SetInteractingActor _asbp_main_guy 0)
  (Variables|/Game/Blueprints/BP_MainGuy.BP_MainGuy_C|SetcanInteract _asbp_main_guy false)
  (Default|HideInteract _asbp_main_guy))

(event EventBeginPlay)

(event Collision|EventActorBeginOverlap
  (params (OtherActor :type Actor%20Object%20Reference)))

(event EventTick
  (params (DeltaSeconds :type Float%20%28single-precision%29)))

(event EventInteract
  (CallFunction|HandleGraveState)
  (if (== (Variables|Default|GetgraveState) 2)
    (bind _asbp_first_person_game_mode (Utilities|Casting|CastToBP_FirstPersonGameMode (Game|GetGameMode)))
    (Default|IsCorrectGrave _asbp_first_person_game_mode (Variables|/Game/FirstPerson/Blueprints/BP_FirstPersonGameMode.BP_FirstPersonGameMode_C|GetcurrentNPC_ID _asbp_first_person_game_mode) (Variables|Default|GetgraveID))
    (Default|SpawnNPC _asbp_first_person_game_mode)))

(fn ConstructionScript
  (Rendering|Components|TextRender|SetText (Variables|Default|GetID) (Utilities|Text|ToText(Integer) (Variables|Default|GetgraveID))))

(fn HandleGraveState
  (bind _player (Variables|Default|Getplayer))
  (switch int (Variables|Default|GetgraveState)
    (:0
      (Rendering|SetVisibility (Variables|Default|GetGroundHole_1) true false)
      (Rendering|SetVisibility (Variables|Debug|GetStaticMeshComponent) false false)
      (Variables|Default|SetgraveState 1))
    (:1
      (if (Variables|/Game/Blueprints/BP_MainGuy.BP_MainGuy_C|GetactiveNPC (Variables|Default|Getplayer))
        (Rendering|SetVisibility (Variables|Debug|GetStaticMeshComponent) true false)
        (Transformation|SetRelativeTransform (Variables|Default|GetGroundHole_1) (Math|Transform|MakeTransform "0.000000,0.000000,-10.000000" "0.000000,90.000000,0.000000" "1.000000,1.000000,1.000000") false false)
        (Rendering|SetVisibility (Variables|Default|GetTombstone_1) true false)
        (Variables|Default|SetgraveState 2)
        (Variables|/Game/Blueprints/BP_MainGuy.BP_MainGuy_C|SetactiveNPC _player false)
        (Default|HideInteract _player)))))