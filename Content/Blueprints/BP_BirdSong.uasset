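; BP_BirdSong is a trigger-volume ambient sound actor that plays bird song when BP_MainGuy enters its box.
; Box overlaps set the AudioActive flag, and entering also starts the sound from the beginning.
; While active, Tick plays a timeline that drives the volume multiplier to ramp the audio up.
; The timeline reverses only if the flag is off when it finishes, and the sound is never explicitly stopped.
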(event OnComponentBeginOverlap(Box)
  (params (OverlappedComponent :type Primitive%20Component%20Object%20Reference) (OtherActor :type Actor%20Object%20Reference) (OtherComp :type Primitive%20Component%20Object%20Reference) (OtherBodyIndex :type Integer) (bFromSweep :type Boolean) (SweepResult :type Hit%20Result%20Structure%20%28by%20ref%29))
  (Utilities|Casting|CastToBP_MainGuy OtherActor)
  (Variables|Default|SetaudioActive true)
  (Audio|Components|Audio|Play (Variables|Default|GetBirdSong) 0.0))

(event OnComponentEndOverlap(Box)
  (params (OverlappedComponent :type Primitive%20Component%20Object%20Reference) (OtherActor :type Actor%20Object%20Reference) (OtherComp :type Primitive%20Component%20Object%20Reference) (OtherBodyIndex :type Integer))
  (Utilities|Casting|CastToBP_MainGuy OtherActor)
  (Variables|Default|SetaudioActive false))

(event EventBeginPlay)

(event Collision|EventActorBeginOverlap
  (params (OtherActor :type Actor%20Object%20Reference)))

(event EventTick
  (params (DeltaSeconds :type Float%20%28single-precision%29))
  (bind _audioactive (Variables|Default|GetaudioActive))
  ;[1 1 1] Cause Audio to ramp up on play
  (if _audioactive
    (bind _audioblend (Timeline|Timeline Play)
      (:Update
        (bind _output_get (Variables|Default|SetcurrentAudioLevel _audioblend))
        (Audio|Components|Audio|SetVolumeMultiplier (Variables|Default|GetBirdSong) _output_get :!class /Script/Engine.AudioComponent))
      (:Finished
        (if (not _audioactive)
          (Timeline|Timeline Reverse))))))

(fn ConstructionScript)